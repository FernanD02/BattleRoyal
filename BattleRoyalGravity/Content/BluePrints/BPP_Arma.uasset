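; Parent weapon Blueprint that manages magazine and reserve ammo for its owning GravityPlayer.
; BeginPlay fills the magazine, sets starting reserves and caches the owner; this, firing and ammo pickup run only on authority.
; Disparando spends a round and triggers Recarga on empty, which flags the player as reloading during a short delay while refilling from reserves.
; AgregarBalas tops up the magazine first, then sends overflow to the capped reserve.
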(event `Recarga`
  (bind _returnvalue (`KismetMathLibrary.Min` (`self.CantidadDeBalasDeRepuesto`) (`self.TamañoDelCargadorDelArma`)))
  (set `/Game/GravityBP/GravityPlayer.EstasRecargando?` true (`self.Jugador`))
  (`KismetSystemLibrary.Delay` 0.2)
  (set `self.CantidadDeBalasEnElArma` _returnvalue)
  (set `self.CantidadDeBalasDeRepuesto` (`KismetMathLibrary.Max` (- (`self.CantidadDeBalasDeRepuesto`) _returnvalue)))
  (set `/Game/GravityBP/GravityPlayer.EstasRecargando?` false (`self.Jugador`)))

(event `Disparando`
  (bind _cantidaddebalasenelarma (`self.CantidadDeBalasEnElArma`))
  (`/Engine/EditorBlueprintResources/ActorMacros.Switch Has Authority`
    (:`Authority`
      (`/Engine/EditorBlueprintResources/StandardMacros.DecrementInt` _cantidaddebalasenelarma
        (:`  `
          (if (<= _cantidaddebalasenelarma 0)
            (if (not (== (+ (`self.CantidadDeBalasEnElArma`) (`self.CantidadDeBalasDeRepuesto`)) 0))
              (`self.Recarga`))))))))

(event `AgregarBalas`
  (params (CantidadDeBalasADar :type Integer))
  (bind _returnvalue (`KismetMathLibrary.Min` CantidadDeBalasADar (- (`self.TamañoDelCargadorDelArma`) (`self.CantidadDeBalasEnElArma`))))
  (bind _returnvalue_2 (- CantidadDeBalasADar _returnvalue))
  (`/Engine/EditorBlueprintResources/ActorMacros.Switch Has Authority`
    (:`Authority`
      (set `self.CantidadDeBalasEnElArma` (+ _returnvalue (`self.CantidadDeBalasEnElArma`)))
      (if (> _returnvalue_2 0)
        (set `self.CantidadDeBalasDeRepuesto` (+ (`KismetMathLibrary.Min` _returnvalue_2 (- (`self.CantidadDeBalasMaximasDeRepuesto`) (`self.CantidadDeBalasDeRepuesto`))) (`self.CantidadDeBalasDeRepuesto`)))))))

(event `self.ReceiveBeginPlay`
  (`/Engine/EditorBlueprintResources/ActorMacros.Switch Has Authority`
    (:`Authority`
      (set `self.CantidadDeBalasEnElArma` (`self.TamañoDelCargadorDelArma`))
      (set `self.CantidadDeBalasDeRepuesto` (`self.CantidadDeBalasConLasQueEmpiezo`))
      (bind _asgravity_player (cast `/Game/GravityBP/GravityPlayer` (`self.GetOwner`)))
      (set `self.Jugador` _asgravity_player))))

(fn `UserConstructionScript`)