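; Base-style pickup actor that spins its mesh and detects when a GravityPlayer enters or leaves its sphere.
; Tick yaws the mesh 180 degrees per second, then zeroes world roll and pitch to keep it upright.
; Sphere overlaps cast to GravityPlayer and call player entered/exited events, which are empty here.
; A hit on the sphere switches off its physics simulation, stopping the pickup where it lands.
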(event `self.ReceiveTick`
  (params (DeltaSeconds :type "Float (single-precision)"))
  (`SceneComponent.K2_AddRelativeRotation` (`self.PickupMesh`) (`KismetMathLibrary.MakeRotator` 0.0 0.0 (* DeltaSeconds 180.0)) false false)
  (`SceneComponent.K2_SetWorldRotation` (`self.PickupMesh`) (`KismetMathLibrary.MakeRotator` 0.0 0.0 (.yaw (`SceneComponent.K2_GetComponentRotation` (`self.PickupMesh`)))) false false))

(event `Pickup_JugadorEntrnado`
  (params (Jugador :type "/Game/GravityBP/GravityPlayer Object Reference")))

(event `Pickup_JugadorSaliendo`
  (params (Jugador :type "/Game/GravityBP/GravityPlayer Object Reference")))

(event `self.PickupSphare.OnComponentBeginOverlap`
  (params (OverlappedComponent :type "PrimitiveComponent Object Reference") (OtherActor :type "Actor Object Reference") (OtherComp :type "PrimitiveComponent Object Reference") (OtherBodyIndex :type Integer) (bFromSweep :type Boolean) (SweepResult :type "HitResult Structure (by ref)"))
  (bind _asgravity_player (cast `/Game/GravityBP/GravityPlayer` OtherActor))
  (`self.Pickup_JugadorEntrnado` _asgravity_player))

(event `self.PickupSphare.OnComponentEndOverlap`
  (params (OverlappedComponent :type "PrimitiveComponent Object Reference") (OtherActor :type "Actor Object Reference") (OtherComp :type "PrimitiveComponent Object Reference") (OtherBodyIndex :type Integer))
  (bind _asgravity_player (cast `/Game/GravityBP/GravityPlayer` OtherActor))
  (`self.Pickup_JugadorSaliendo` _asgravity_player))

(event `self.PickupSphare.OnComponentHit`
  (params (HitComponent :type "PrimitiveComponent Object Reference") (OtherActor :type "Actor Object Reference") (OtherComp :type "PrimitiveComponent Object Reference") (NormalImpulse :type "Vector Structure") (Hit :type "HitResult Structure (by ref)"))
  (`PrimitiveComponent.SetSimulatePhysics` (`self.PickupSphare`) false))

(fn `UserConstructionScript`)