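; BP_Salud_Pickup is a health pickup that heals the player who enters it.
; Its PickupJugadorEntrnado event runs only on authority and checks that the player's SaludDelPersonaje is below SlaudMaxima.
; If so, it passes a negated CantidadDeSalud to the player's ModificarSalud and destroys itself.
; At full health the pickup stays in the world.
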(event `self.Pickup_JugadorEntrnado`
  (params (Jugador :type "/Game/GravityBP/GravityPlayer Object Reference"))
  (`/Engine/EditorBlueprintResources/ActorMacros.Switch Has Authority`
    (:`Authority`
      (if (< (`/Game/GravityBP/GravityPlayer.SaludDelPersonaje` Jugador) (`/Game/GravityBP/GravityPlayer.SlaudMaxima` Jugador))
        (`/Game/GravityBP/GravityPlayer.ModificarSalud` Jugador (* (`self.CantidadDeSalud`) -1))
        (`self.K2_DestroyActor`)))))

(fn `UserConstructionScript`
  (`parent.UserConstructionScript`))