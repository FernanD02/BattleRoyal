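; Weapon pickup actor that players can collect, carrying the assigned weapon class and its ammunition.
; On BeginPlay the server copies magazine and reserve ammo counts from the assigned weapon's class defaults.
; Enter and exit events register this pickup as the player's current ArmaPickUp, clearing it on exit only if it still points here.
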(event `self.ReceiveBeginPlay`
  (bind (_cantidaddebalasenelarma `_tamañodelcargadordelarma` _cantidaddebalasderepuesto) (defaults `/Game/BluePrints/PickUp/BP_Arma_PickUp` (`self.ArmaAsignar`)))
  (`/Engine/EditorBlueprintResources/ActorMacros.Switch Has Authority`
    (:`Authority`
      (set `self.BalasQueTiraElCargador` _cantidaddebalasenelarma)
      (set `self.BalasDeRespuesto` _cantidaddebalasderepuesto))))

(event `self.Pickup_JugadorEntrnado`
  (params (Jugador :type "/Game/GravityBP/GravityPlayer Object Reference"))
  (set `/Game/GravityBP/GravityPlayer.ArmaPickUp` self Jugador))

(event `self.Pickup_JugadorSaliendo`
  (params (Jugador :type "/Game/GravityBP/GravityPlayer Object Reference"))
  (if (== (`/Game/GravityBP/GravityPlayer.ArmaPickUp` Jugador) self)
    (set `/Game/GravityBP/GravityPlayer.ArmaPickUp` null Jugador)))

(fn `UserConstructionScript`
  (`parent.UserConstructionScript`))