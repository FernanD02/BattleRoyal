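; Ball actor that travels along the spline of a referenced track actor, starting automatically on BeginPlay.
; The BallMover timeline has its play rate set from Duration and its start time from BallStartOffset.
; Each update maps the timeline's Alpha to a distance along MySpline and applies that point's world location and rotation to the ball.
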(event `self.ReceiveBeginPlay`
  (`self.MoveBall`))

(event `MoveBall`
  (bind _returnvalue (`KismetMathLibrary.Lerp` 0.0 (`SplineComponent.GetSplineLength` (`/Game/Nivel/NivelBluePrints/BallTrack_BP.MySpline` (`self.TrackReferance`))) (`self.Alpha`)))
  (`TimelineComponent.SetPlayRate` (`self.BallMover`) (/ 1.0 (`self.Duration`)))
  (`TimelineComponent.SetNewTime` (`self.BallMover`) (`self.BallStartOffset`))
  (bind (_direction _alpha) (`Timeline|BallMover`)
    (:`Update`
      (set `self.Alpha` _alpha)
      (`self.K2_SetActorLocationAndRotation` (`SplineComponent.GetLocationAtDistanceAlongSpline` (`/Game/Nivel/NivelBluePrints/BallTrack_BP.MySpline` (`self.TrackReferance`)) _returnvalue "World") (`SplineComponent.GetRotationAtDistanceAlongSpline` (`/Game/Nivel/NivelBluePrints/BallTrack_BP.MySpline` (`self.TrackReferance`)) _returnvalue "World")))))

(fn `UserConstructionScript`)